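; Player character Blueprint with a Space-triggered forward dash and a Health value that drains each Tick and prints as debug output.
; DashSetup temporarily overrides movement acceleration, speed and rotation rate, then restores values cached at BeginPlay; both calls keep the mesh visible.
; A timeline drives forward input and a slight camera FOV change while input is disabled.
; Niagara dash FX runs throughout, switching off shortly after the dash ends.
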(event EventBeginPlay
  (bind _charactermovement (Variables|Character|GetCharacterMovement))
  (bind _dashrate (Variables|Default|GetDashRate))
  (Variables|Default|SetMax%20Acceleration (Variables|/Script/Engine.CharacterMovementComponent|GetMaxAcceleration _charactermovement))
  (Variables|Default|SetMax%20Walk%20Speed (Variables|/Script/Engine.CharacterMovementComponent|GetMaxWalkSpeed _charactermovement))
  (Variables|Default|SetRotation%20Rate (Variables|/Script/Engine.CharacterMovementComponent|GetRotationRate _charactermovement))
  (Components|Timeline|SetPlayRate (Variables|Default|GetDashTimeline) _dashrate)
  (Variables|Default|SetDashSpeed (* _dashrate (Variables|Default|GetDashDistance))))

(event EventTick
  (params (DeltaSeconds :type Float%20%28single-precision%29))
  (Variables|Default|SetHealth (- (Variables|Default|GetHealth) DeltaSeconds))
  (Development|PrintString (Utilities|String|ToString(Float) (Variables|Default|GetHealth))))

(event Input|KeyboardEvents|SpaceBar
  (params (Key :type Key%20Structure :default "None"))
  (:Pressed
    (Input|DisableInput (Game|GetPlayerController 0))
    (Utilities|DashSetup 1e+08 (Variables|Default|GetDashSpeed) "0,10000000.000000,0" true)
    (Components|Activation|SetActive (Variables|Default|GetNS_Dash_FX) true false)
    (bind _newtrack_0 (Timeline|DashTimeline PlayFromStart)
      (:Update
        (Pawn|Input|AddMovementInput (Transformation|GetActorForwardVector) 1.0 false)
        (Camera|SetFieldOfView (Variables|Default|GetCameraComp) (Math|Float|Lerp 55.0 6e+01 _newtrack_0)))
      (:Finished
        (Utilities|DashSetup (Variables|Default|GetMax%20Acceleration) (Variables|Default|GetMax%20Walk%20Speed) (Variables|Default|GetRotation%20Rate) true)
        (Input|EnableInput (Game|GetPlayerController 0))
        (Utilities|FlowControl|Delay 0.06)
        (Components|Activation|SetActive (Variables|Default|GetNS_Dash_FX) false false)))))

(fn ConstructionScript)