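; BP_Folder is an enemy Blueprint that plays a telegraphed "fool" attack display.
; Its FoolAttack event prints a debug string, blinks the WarningAttack component twice through timed delays, then briefly shows the YouFool component before hiding it.
; The sequence only toggles component visibility, with no damage or collision logic, and nothing in this file calls the event.
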(event Custom|FoolAttack
  (Development|PrintString "fool")
  (Rendering|SetVisibility (Variables|Default|GetWarningAttack) true false)
  (Utilities|FlowControl|Delay 0.3)
  (Rendering|SetVisibility (Variables|Default|GetWarningAttack) false false)
  (Utilities|FlowControl|Delay 0.3)
  (Rendering|SetVisibility (Variables|Default|GetWarningAttack) true false)
  (Utilities|FlowControl|Delay 0.3)
  (Rendering|SetVisibility (Variables|Default|GetWarningAttack) false false)
  (Utilities|FlowControl|Delay 0.3)
  (Rendering|SetVisibility (Variables|Default|GetYouFool) true false)
  (Utilities|FlowControl|Delay 1.0)
  (Rendering|SetVisibility (Variables|Default|GetYouFool) false false))

(event EventBeginPlay)

(event Collision|EventActorBeginOverlap
  (params (OtherActor :type Actor%20Object%20Reference)))

(event EventTick
  (params (DeltaSeconds :type Float%20%28single-precision%29)))

(fn ConstructionScript)