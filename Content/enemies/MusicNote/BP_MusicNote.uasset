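; BP_MusicNote is an enemy actor, a music note that performs a telegraphed area-of-effect attack.
; Its AoeAttack event blinks the WarningAttack component twice through a chain of short delays, then spawns BP_AoeAttack at the note's own transform.
; Nothing in this Blueprint calls the event, as BeginPlay, overlap, Tick and the construction script are empty.
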(event Custom|AoeAttack
  (Rendering|SetVisibility (Variables|Default|GetWarningAttack) true false)
  (Utilities|FlowControl|Delay 0.3)
  (Rendering|SetVisibility (Variables|Default|GetWarningAttack) false false)
  (Utilities|FlowControl|Delay 0.3)
  (Rendering|SetVisibility (Variables|Default|GetWarningAttack) true false)
  (Utilities|FlowControl|Delay 0.3)
  (Rendering|SetVisibility (Variables|Default|GetWarningAttack) false false)
  (Utilities|FlowControl|Delay 0.3)
  (Game|SpawnActorfromClass "/Game/enemies/MusicNote/BP_AoeAttack.BP_AoeAttack_C" (Transformation|GetActorTransform) "Undefined" 0 0))

(event EventBeginPlay)

(event Collision|EventActorBeginOverlap
  (params (OtherActor :type Actor%20Object%20Reference)))

(event EventTick
  (params (DeltaSeconds :type Float%20%28single-precision%29)))

(fn ConstructionScript)