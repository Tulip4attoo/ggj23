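; Short-lived area attack actor, filed under the MusicNote enemy, that damages the player on overlap.
; BeginPlay activates the Niagara effect, clears the MakeDam flag after a brief delay, then destroys the actor about 1.5 seconds later.
; A StaticMesh overlap with BP_Main prints a debug string and applies SkillDam only while MakeDam is set, so the damage window is shorter than the actor's lifetime.
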(event OnComponentBeginOverlap(StaticMesh)
  (params (OverlappedComponent :type Primitive%20Component%20Object%20Reference) (OtherActor :type Actor%20Object%20Reference) (OtherComp :type Primitive%20Component%20Object%20Reference) (OtherBodyIndex :type Integer) (bFromSweep :type Boolean) (SweepResult :type Hit%20Result%20Structure%20%28by%20ref%29))
  (bind _asbp_main (Utilities|Casting|CastToBP_Main OtherActor))
  (Development|PrintString "Hello")
  (if (Variables|Default|GetMakeDam?)
    (Game|Damage|ApplyDamage _asbp_main (Variables|Default|GetSkillDam) 0 0)))

(event EventBeginPlay
  (Components|Activation|SetActive (Variables|Default|GetNiagara) true false)
  (Utilities|FlowControl|Delay 0.2)
  (Variables|Default|SetMakeDam? false)
  (Utilities|FlowControl|Delay 1.5)
  (Actor|DestroyActor))

(fn ConstructionScript)